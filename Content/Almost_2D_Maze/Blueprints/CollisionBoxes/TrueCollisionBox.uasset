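; TrueCollisionBox is a collision actor in the Almost 2D Maze game that responds to overlaps with sound and a flash of light.
; On begin overlap, with no check on the other actor, it plays its audio and raises the spotlight to the highest intensity unless already brighter.
; Tick steps the intensity down by a fixed amount each frame while above the medium level, so the fade depends on frame rate.
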(event Collision|EventActorBeginOverlap
  (params (OtherActor :type Actor%20Object%20Reference))
  (Audio|Components|Audio|Play (Variables|Default|GetAudio) 0.0)
  (if (<= (Variables|/Script/Engine.LightComponentBase|GetIntensity (Variables|Default|GetSpotLight)) (Variables|Default|GetHighest_Intensity))
    (Rendering|Components|Light|SetIntensity (Variables|Default|GetSpotLight) (Variables|Default|GetHighest_Intensity))))

(event EventTick
  (params (DeltaSeconds :type Float%20%28single-precision%29))
  (bind _spotlight (Variables|Default|GetSpotLight))
  (if (not (<= (Variables|/Script/Engine.LightComponentBase|GetIntensity (Variables|Default|GetSpotLight)) (Variables|Default|GetMediumIntensity)))
    (Rendering|Components|Light|SetIntensity _spotlight (- (Variables|/Script/Engine.LightComponentBase|GetIntensity _spotlight) 5e+02))))

(fn ConstructionScript)