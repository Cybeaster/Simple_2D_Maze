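; Player controller for click-to-move navigation that sends the controlled pawn toward the point under the cursor.
; Holding SetDestination opens a gate that lets Tick repeatedly trace under the cursor and call MoveToHitLocation.
; MoveToHitLocation issues SimpleMoveToLocation only when the hit is closer to the pawn than MinDistance.
; Touch1 toggles a second gate with the same cursor trace, but nothing feeds that gate's Enter.
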(event EventTick
  (params (DeltaSeconds :type Float%20%28single-precision%29))
  (Utilities|FlowControl|Sequence
    (:then_0
      (Utilities|FlowControl|Gate true
        (:Exit
          (CallFunction|MovetoHitLocation (.HitResult (Game|Player|GetHitResultUnderCursorbyChannel "TraceTypeQuery1" true))))))))

(event Input|ActionEvents|InputActionSetDestination
  (params (Key :type Key%20Structure :default "None"))
  (:Pressed
    (Utilities|FlowControl|Gate true) ; enters at Open
  )
  (:Released
    (Utilities|FlowControl|Gate true) ; enters at Close
  ))

(event Input|TouchEvents|InputTouch
  (params (Location :type Vector) (FingerIndex :type ETouchIndex%20Enum))
  (bind _returnvalue (Utilities|Enum|Equal(Enum) FingerIndex "Touch1"))
  (:Pressed
    (if _returnvalue
      (Utilities|FlowControl|Gate true :!label _label ; enters at Open
        (:Exit
          (CallFunction|MovetoHitLocation (.HitResult (Game|Player|GetHitResultUnderCursorbyChannel "TraceTypeQuery1" true)))))))
  (:Released
    (if _returnvalue
      (goto _label Close))))

(fn ConstructionScript)

(fn MovetoHitLocation
  (params (Hit :type Hit%20Result%20Structure))
  (bind _location (Collision|BreakHitResult Hit))
  (if (not (>= (Math|Vector|VectorLength (- (Transformation|GetActorLocation (Pawn|GetControlledPawn)) _location)) (Variables|Default|GetMinDistance)))
    (AI|Navigation|SimpleMovetoLocation self _location)))